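; Keypad puzzle actor that opens the fence door when the player enters the correct button sequence, then quits the game ten seconds later.
; Interacting freezes player movement and shows a WBP_Buttons widget with UI-only input and a mouse cursor.
; The widget receives the keypad reference, and ButtonPressed checks each press against the ordered code, resetting progress on a mistake.
; Success removes the widget, re-enables movement and opens the BP_FenceDoor found at BeginPlay.
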(event Custom|delayClose
  (Utilities|FlowControl|Delay 1e+01)
  (Game|QuitGame 0 "Quit" false))

(event EventBeginPlay
  (bind _returnvalue (Actor|GetActorOfClass "/Game/Blueprints/Interactions/BP_FenceDoor.BP_FenceDoor_C"))
  (Variables|Default|SetDoorReference _returnvalue))

(event Collision|EventActorBeginOverlap
  (params (OtherActor :type Actor%20Object%20Reference)))

(event EventTick
  (params (DeltaSeconds :type Float%20%28single-precision%29)))

(event EventInteract
  (bind _returnvalue (Game|GetPlayerController 0))
  (bind _asbp_player_character (Utilities|Casting|CastToBP_PlayerCharacter (Game|GetPlayerCharacter 0)))
  (Default|DisableMovement _asbp_player_character)
  (bind _returnvalue_2 (UserInterface|CreateWidget "/Game/Blueprints/Puzzle/WBP_Buttons.WBP_Buttons_C" 0 self))
  (bind _output_get (Variables|Default|SetPuzzleWidget _returnvalue_2))
  (UserInterface|Viewport|AddtoViewport _output_get 0)
  (Input|SetInputModeUIOnly _returnvalue 0 "DoNotLock" false)
  (Variables|/Script/Engine.PlayerController|SetbShowMouseCursor _returnvalue true))

(fn ConstructionScript)

(fn ButtonPressed
  (params (PressedButton :type Integer))
  (Audio|PlaySound2D "/Game/Sounds/buttonClick.buttonClick" 1.0 1.0 0.0 0 0)
  (if (== PressedButton (Utilities|Array|Get(acopy) (Variables|Default|GetCorrectButtonOrder) (Variables|Default|GetactualButton)))
    (bind _output_get (Variables|Default|SetactualButton (+ (Variables|Default|GetactualButton) 1)))
    (if (>= _output_get 4)
      (Audio|PlaySound2D "/Game/Sounds/open_fence.open_fence" 1.0 1.0 0.0 0 0)
      (Default|CallOnPuzzleSolved)
      (Widget|RemovefromParent (Variables|Default|GetPuzzleWidget))
      (bind _asbp_player_character (Utilities|Casting|CastToBP_PlayerCharacter (Game|GetPlayerCharacter 0)))
      (Default|EnableMovement _asbp_player_character)
      (Default|OpenDoor (Variables|Default|GetDoorReference))
      (CallFunction|DelayClose))
    (else
      (Variables|Default|SetactualButton 0)
      (Development|PrintText "Error")
      (Audio|PlaySound2D "/Game/Sounds/soundError.soundError" 1.0 1.0 0.0 0 0))))