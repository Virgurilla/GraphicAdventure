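; Player character Blueprint with Enhanced Input movement and look, interaction through BPI_Interactable, and dialogue control.
; A short camera line trace runs on interact to message the hit actor, and every Tick to show the prompt widget.
; The prompt hides only when the trace hits nothing, not on non-interactable hits.
; StartDialogue opens WBP_Dialogue with given lines, disabling movement and switching to UI-only input; EndDialogue removes it and restores control.
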(event Input|EnhancedActionEvents|EnhancedInputActionIA_Move
  (params (ActionValue :type Vector%202D%20Structure) (ElapsedSeconds :type Float%20%28double-precision%29) (TriggeredSeconds :type Float%20%28double-precision%29) (InputAction :type Input%20Action%20Object%20Reference :default "/Game/Blueprints/Core/Input/IA_Move.IA_Move"))
  (bind (_x _y) (Math|Vector2D|BreakVector2D ActionValue))
  (bind _returnvalue (Pawn|GetControlRotation :!class /Script/Engine.Pawn))
  (bind _yaw (Math|Rotator|BreakRotator _returnvalue))
  (bind _returnvalue_2 (Math|Rotator|MakeRotator 0.0 0.0 _yaw))
  ;[0.15 0.15 0.15 0.5] Player Movement
  (Pawn|Input|AddMovementInput (Math|Vector|GetRightVector _returnvalue_2) _x false)
  (Pawn|Input|AddMovementInput (Math|Vector|GetForwardVector _returnvalue_2) _y false))

(event Input|EnhancedActionEvents|EnhancedInputActionIA_Look
  (params (ActionValue :type Vector%202D%20Structure) (ElapsedSeconds :type Float%20%28double-precision%29) (TriggeredSeconds :type Float%20%28double-precision%29) (InputAction :type Input%20Action%20Object%20Reference :default "/Game/Blueprints/Core/Input/IA_Look.IA_Look"))
  (bind (_x _y) (Math|Vector2D|BreakVector2D ActionValue))
  ;[0.15 0.15 0.15 0.5] Player Camera
  (Pawn|Input|AddControllerYawInput _x)
  (Pawn|Input|AddControllerPitchInput _y))

(event Input|EnhancedActionEvents|EnhancedInputActionIA_Interact
  (params (ActionValue :type Boolean) (ElapsedSeconds :type Float%20%28double-precision%29) (TriggeredSeconds :type Float%20%28double-precision%29) (InputAction :type Input%20Action%20Object%20Reference :default "/Game/Blueprints/Core/Input/IA_Interact.IA_Interact"))
  (bind _camera (Variables|Default|GetCamera))
  (bind _returnvalue (Transformation|GetWorldLocation _camera))
  ;[0.15 0.15 0.15 0.5] Player Interaction RayCast
  (:Started
    (bind (_outhit _returnvalue_2) (Collision|LineTraceByChannel _returnvalue (+ _returnvalue (* (Math|Vector|GetForwardVector _camera) (Math|Float|MakeLiteralFloat 4e+02))) "TraceTypeQuery1" false 0 "None"))
    (if _returnvalue_2
      (if (Utilities|DoesObjectImplementInterface (.HitActor (Collision|BreakHitResult _outhit)) "/Game/Blueprints/Interactions/BPI_Interactable.BPI_Interactable_C")
        (Class|BPIInteractable|Interact(Message) (.HitActor (Collision|BreakHitResult _outhit)))))))

(event EventBeginPlay
  ;[0.15 0.15 0.15 0.5] Mapping Context
  (bind _asplayer_controller (Utilities|Casting|CastToPlayerController (Pawn|GetController)))
  (Input|AddMappingContext (PlayerController|LocalPlayerSubsystems|GetEnhancedInputLocalPlayerSubsystem _asplayer_controller) "/Game/Blueprints/Core/Input/IMC_Player.IMC_Player" 0 "(bIgnoreAllPressedKeysUntilRelease=True,bForceImmediately=False,bNotifyUserSettings=False)")
  ;[0.15 0.15 0.15 0.5] Create Interaction Widget
  (bind _returnvalue (UserInterface|CreateWidget "/Game/Blueprints/UI/WBP_InteractPrompt.WBP_InteractPrompt_C"))
  (UserInterface|Viewport|AddtoViewport _returnvalue 0)
  (Widget|SetVisibility _returnvalue "Hidden")
  (Variables|Default|SetInteractPromptWidget _returnvalue))

(event EventTick
  (params (DeltaSeconds :type Float%20%28single-precision%29))
  ;[0.15 0.15 0.15 0.5] Check for Interactable per tick
  (CallFunction|CheckforInteractable))

(fn ConstructionScript)

(fn StartDialogue
  (params (DialogueLines :type Array%20of%20ST%20Dialogue%20Line%20Structures))
  ;[0.15 0.15 0.15 0.5] Start dialogue Widget and disable movement
  (bind _asplayer_controller (Utilities|Casting|CastToPlayerController (Pawn|GetController)))
  (bind _returnvalue (UserInterface|CreateWidget "/Game/Blueprints/UI/WBP_Dialogue.WBP_Dialogue_C" _asplayer_controller))
  (bind _output_get (Variables|Default|SetDialogueWidget _returnvalue))
  (Variables|/Game/Blueprints/UI/WBP_Dialogue.WBP_Dialogue_C|SetDialogueLines _output_get DialogueLines)
  (UserInterface|Viewport|AddtoViewport _output_get 0)
  (CallFunction|DisableMovement)
  (Input|SetInputModeUIOnly _asplayer_controller _output_get "DoNotLock" false)
  (Variables|/Script/Engine.PlayerController|SetbShowMouseCursor _asplayer_controller true))

(fn DisableMovement
  (Pawn|Components|CharacterMovement|DisableMovement (Variables|Character|GetCharacterMovement)))

(fn EnableMovement
  (Pawn|Components|CharacterMovement|SetMovementMode (Variables|Character|GetCharacterMovement) "MOVE_Walking" 0)
  (bind _asplayer_controller (Utilities|Casting|CastToPlayerController (Pawn|GetController)))
  (Input|SetInputModeGameOnly _asplayer_controller false)
  (Variables|/Script/Engine.PlayerController|SetbShowMouseCursor _asplayer_controller false))

(fn EndDialogue
  (Widget|RemovefromParent (Variables|Default|GetDialogueWidget))
  (CallFunction|EnableMovement))

(fn CheckforInteractable
  (bind _camera (Variables|Default|GetCamera))
  (bind _returnvalue (Transformation|GetWorldLocation _camera))
  ;[0.15 0.15 0.15 0.5] Trace line per tick
  (bind (_outhit _returnvalue_2) (Collision|LineTraceByChannel _returnvalue (+ _returnvalue (* (Math|Vector|GetForwardVector _camera) (Math|Float|MakeLiteralFloat 4e+02))) "TraceTypeQuery1" false 0 "None"))
  (if _returnvalue_2
    ;[0.15 0.15 0.15 0.5] Interactable found (show widget)
    (if (Utilities|DoesObjectImplementInterface (.HitActor (Collision|BreakHitResult _outhit)) "/Game/Blueprints/Interactions/BPI_Interactable.BPI_Interactable_C")
      (Widget|SetVisibility (Variables|Default|GetInteractPromptWidget) "Visible"))
    (else
      ;[0.15 0.15 0.15 0.5] No interactable found (hide widget)
      (Widget|SetVisibility (Variables|Default|GetInteractPromptWidget) "Hidden"))))